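; BP_BloodSystemComponent holds a Blood resource, clamped between zero and MaxBlood, with functions to gain and spend it.
; GainBlood adds a Damage value and plays a 2D hit sound whose volume and pitch rise with the current Blood level.
; SpendBlood deducts an amount only when enough Blood is available, and otherwise does nothing without reporting failure.
; The event graph has no active logic.
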(fn `GainBlood`
  (params (Damage :type "Float (double-precision)"))
  (bind _output_get (set `self.Blood` (`KismetMathLibrary.FClamp` (+ Damage (`self.Blood`)) 0.0 (`self.MaxBlood`))))
  (bind _returnvalue (+ (/ _output_get 50.0) (`self.BloodSFXMult`)))
  (`GameplayStatics.PlaySound2D` "/Game/_Game/Audio/SFX/BloodHit.BloodHit" _returnvalue _returnvalue 0.0 null null))

(fn `SpendBlood`
  (params (Amount :type "Float (double-precision)"))
  (if (<= Amount (`self.Blood`))
    (set `self.Blood` (`KismetMathLibrary.FClamp` (- (`self.Blood`) Amount) 0.0 (`self.MaxBlood`)))))