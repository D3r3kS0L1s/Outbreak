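; Health component that tracks an actor's health, reacts to damage and healing, and broadcasts OnKilled at zero.
; It binds to the owner's any-damage event, clamps health and plays hit or kill sound and Niagara effects.
; Damage to a BP_Enemy owner grants blood to the damage causer's blood system component.
; Healing always flashes the first player's HUD, with a burst effect and heal and heartbeat sounds.
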(event `self.ReceiveBeginPlay`
  (set `self.Owner` (`self.GetOwner`))
  (set `self.Health` (`self.MaxHealth`))
  (add `Actor.OnTakeAnyDamage` (`self.Owner`) (`|CreateDelegate` :!event `TookDamage`)))

(event `TookDamage`
  (params (DamagedActor :type "Actor Object Reference") (Damage :type "Float (single-precision)") (DamageType :type "DamageType Object Reference") (InstigatedBy :type "Controller Object Reference") (DamageCauser :type "Actor Object Reference"))
  (set `self.Health` (`KismetMathLibrary.FClamp` (- (`self.Health`) Damage) 0.0 (`self.MaxHealth`)))
  (if (<= (`self.Health`) 0.0)
    (`self.PlayFx` (`self.KillSound`) (`self.KillParticles`))
    (if (== (`GameplayStatics.GetObjectClass` (`self.GetOwner`)) "/Game/_Game/Gameplay/BP_Enemy.BP_Enemy_C")
      (`/Game/_Game/Blueprints/Components/BP_BloodSystemComponent.GainBlood` (`Actor.GetComponentByClass` DamageCauser "/Game/_Game/Blueprints/Components/BP_BloodSystemComponent.BP_BloodSystemComponent_C") Damage)
      (`self.OnKilled`)
      (else
        (`self.OnKilled`)))
    (else
      (`self.PlayFx` (`self.DamagedSound`) (`self.DamageParticles`))
      (if (== (`GameplayStatics.GetObjectClass` (`self.GetOwner`)) "/Game/_Game/Gameplay/BP_Enemy.BP_Enemy_C")
        (`/Game/_Game/Blueprints/Components/BP_BloodSystemComponent.GainBlood` (`Actor.GetComponentByClass` DamageCauser "/Game/_Game/Blueprints/Components/BP_BloodSystemComponent.BP_BloodSystemComponent_C") Damage)))))

(event `Healed`
  (params (Amount :type "Float (double-precision)"))
  (set `self.Health` (`KismetMathLibrary.FClamp` (+ Amount (`self.Health`)) 0.0 (`self.MaxHealth`)))
  (bind _asbp_first_person_player_controller (cast `/Game/FirstPerson/Blueprints/BP_FirstPersonPlayerController` (`GameplayStatics.GetPlayerController` 0)))
  (bind _player_hud_widget (`/Game/FirstPerson/Blueprints/BP_FirstPersonPlayerController.Player HUD Widget` _asbp_first_person_player_controller))
  (`UserWidget.PlayAnimation` _player_hud_widget (`/Game/_Game/UI/WBP_PlayerHUD.HealScreenFlashAnimation` _player_hud_widget) 0.0 1 "Forward" 1.0 false)
  (`NiagaraFunctionLibrary.SpawnSystemAtLocation` "/Game/_Game/VFX/Particles/PS_HealBurst.PS_HealBurst" (`Actor.K2_GetActorLocation` (`self.GetOwner`)))
  (`GameplayStatics.PlaySound2D` "/Game/_Game/Audio/SFX/664265__silverillusionist__healing-balm_Cue.664265__silverillusionist__healing-balm_Cue" 1.0 1.0 0.0 null null)
  (`KismetSystemLibrary.Delay` 0.3)
  (`GameplayStatics.PlaySound2D` "/Game/_Game/Audio/SFX/564013__rlkhafi__heart_beat_Cue.564013__rlkhafi__heart_beat_Cue" 1.0 1.0 0.0 null null))

(fn `Kill`)

(fn `PlayFx`
  (params (SFX :type "SoundBase Object Reference") (VFX :type "NiagaraSystem Object Reference"))
  (bind _returnvalue (`Actor.K2_GetActorLocation` (`self.Owner`)))
  (`GameplayStatics.PlaySoundAtLocation` SFX _returnvalue (struct) 1.0 1.0 0.0 null null null null)
  (`NiagaraFunctionLibrary.SpawnSystemAtLocation` VFX (+ _returnvalue (0.0 0.0 150.0))))