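; BP_Enemy is an enemy actor that shoots projectiles at the first-person player when it sees them.
; On PawnSensing sight, it yaws toward the player and aims its projectile spawn point with full pitch.
; It then spawns BP_EnemyProjectile with a fire-spell sound, gated by a one-second CanAttack cooldown.
; Its health system component's OnKilled event destroys the actor.
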(event `self.ReceiveBeginPlay`
  (add `/Game/_Game/Blueprints/Components/BP_HealthSystemComponent.OnKilled` (`self.BP_HealthSystemComponent`) (delegate `OnKilled`)))

(event `OnKilled`
  (`self.K2_DestroyActor`))

(event `self.PawnSensing.OnSeePawn`
  (params (Pawn :type "Pawn Object Reference"))
  (bind _asbp_first_person_character (cast `/Game/FirstPerson/Blueprints/BP_FirstPersonCharacter` Pawn))
  (bind (_returnvalue_roll _returnvalue_pitch _returnvalue_yaw) (`KismetMathLibrary.BreakRotator` (`KismetMathLibrary.FindRelativeLookAtRotation` (`KismetMathLibrary.Conv_VectorToTransform` (`self.K2_GetActorLocation`)) (`self.K2_GetActorLocation` _asbp_first_person_character))))
  (`self.K2_SetActorRotation` (`KismetMathLibrary.MakeRotator` _returnvalue_roll 0.0 _returnvalue_yaw))
  (`SceneComponent.K2_SetWorldRotation` (`self.SpawnProjectileLocation`) (`KismetMathLibrary.MakeRotator` _returnvalue_roll _returnvalue_pitch _returnvalue_yaw) false false)
  (if (`self.CanAttack?`)
    (`|SpawnActorFromClass` "/Game/_Game/Gameplay/BP_EnemyProjectile.BP_EnemyProjectile_C" (`SceneComponent.K2_GetComponentToWorld` (`self.SpawnProjectileLocation`)) "Undefined" "MultiplyWithRoot" null null)
    (`GameplayStatics.PlaySoundAtLocation` "/Game/_Game/Audio/SFX/541478__eminyildirim__magic-fire-spell-impact-punch_Cue.541478__eminyildirim__magic-fire-spell-impact-punch_Cue" (`self.K2_GetActorLocation`) (struct) 1.0 1.0 0.0 null null null null)
    (set `self.CanAttack?` false)
    (`KismetSystemLibrary.Delay` 1.0)
    (set `self.CanAttack?` true)))

(fn `UserConstructionScript`)